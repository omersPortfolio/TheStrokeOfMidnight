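; BP_MaynardChasing is the chasing variant of the Maynard AI enemy, exposing movement speed, attack and attack range to its controlling logic.
; Attack plays a full-body montage whose notify switches the hand collider to overlap Pawns, opening the hit window.
; A fixed delay, triggered on montage start or interruption rather than completion, then clears the Attacked flag and sets the collider back to ignore Pawns.
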(event EventSetMovementSpeed
  (params (NewSpeed :type Float%20%28single-precision%29))
  ;[0.609 0.7279 1 1 37] Interface Functions
  (Variables|/Script/Engine.CharacterMovementComponent|SetMaxWalkSpeed (Variables|Character|GetCharacterMovement) NewSpeed))

(event EventAttack
  (bind _handcollider (Variables|Default|GetHandCollider))
  ;[0.609 0.7279 1 1 37] Interface Functions
  (Animation|Montage|PlayMontage (Variables|Character|GetMesh) "/Game/Enemies/Maynard/Animations/SingleAnimations/Attack/AM_MaynardAttack_FullBody.AM_MaynardAttack_FullBody" 1.0 0.0 "Start"
    (:then
      (Utilities|FlowControl|Delay 1.65 :!label _label)
      (Variables|Default|SetbAttacked false)
      (Collision|SetCollisionResponsetoChannel _handcollider "ECC_Pawn" "ECR_Ignore"))
    (:OnInterrupted
      (goto _label))
    (:OnNotifyBegin
      (Collision|SetCollisionResponsetoChannel _handcollider "ECC_Pawn" "ECR_Overlap"))))

(fn ConstructionScript)

(fn GetAttackRange
  (return (Variables|Default|GetAttackRange)))