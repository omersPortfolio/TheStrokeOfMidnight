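; BP_AIMaynard is the AI-controlled Maynard character, exposing its patrol path, attack range and identity checks through interface functions.
; State changes are forwarded to the animation instance, and walk speed is set per state from passive to attacking or directly by value.
; Attacks play a montage whose notify switches the hand collider to overlap pawns.
; A short delay after play starts or is interrupted resets the attack flag and collider.
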(event EventSetMovementSpeed
  (params (NewSpeed :type Float%20%28single-precision%29))
  ;[0.6159 0.7401 1 1 37] Interface Functions
  (Variables|/Script/Engine.CharacterMovementComponent|SetMaxWalkSpeed (Variables|Character|GetCharacterMovement) NewSpeed))

(event EventNotifyStateChanged
  (params (NewState :type EAIState%20Enum :default "Passive"))
  ;[0.6159 0.7401 1 1 37] Interface Functions
  (Class|INTAIHelper|NotifyStateChanged(Message) (Components|SkeletalMesh|GetAnimInstance (Variables|Character|GetMesh)) NewState))

(event EventUpdateMovementSpeed
  (params (State :type EAIState%20Enum :default "Passive"))
  ;[0.6159 0.7401 1 1 37] Interface Functions
  (Variables|/Script/Engine.CharacterMovementComponent|SetMaxWalkSpeed (Variables|Character|GetCharacterMovement) (Utilities|Select :Index State :Passive 1.8e+02 :Investigating 2.4e+02 :Seeking 2.5e+02 :Attacking 275.0)))

(event EventAttack
  (bind _handcollider (Variables|Default|GetHandCollider))
  ;[0.6159 0.7401 1 1 37] Interface Functions
  (Animation|Montage|PlayMontage (Variables|Character|GetMesh) "/Game/Enemies/Maynard/Animations/SingleAnimations/Attack/AM_MaynardAttack.AM_MaynardAttack" 1.0 0.0 "Start"
    (:then
      (Utilities|FlowControl|Delay 1.65 :!label _label)
      (Variables|Default|SetbAttacked false)
      (Collision|SetCollisionResponsetoChannel _handcollider "ECC_Pawn" "ECR_Ignore"))
    (:OnInterrupted
      (goto _label))
    (:OnNotifyBegin
      (Collision|SetCollisionResponsetoChannel _handcollider "ECC_Pawn" "ECR_Overlap"))))

(fn ConstructionScript)

(fn IsDead
  (return false))

(fn IsActorPlayer
  (return false))

(fn GetPatrolPath
  (return (Variables|Default|GetPatrolPath)))

(fn GetAttackRange
  (return (Variables|Default|GetAttackRange)))