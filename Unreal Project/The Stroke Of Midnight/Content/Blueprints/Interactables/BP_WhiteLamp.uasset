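; BP_WhiteLamp is a lamp that flickers randomly during play.
; From BeginPlay, a self-repeating loop with a very short Delay compares a random integer against FlickerFrequency on each pass.
; Light and PointLight are shown when the roll meets or exceeds that value and hidden otherwise, so higher FlickerFrequency values keep the lamp dark more often.
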(event EventBeginPlay
  (bind _light (Variables|Default|GetLight))
  (bind _pointlight (Variables|Default|GetPointLight))
  (Math|Integer|CompareInt (Math|Random|RandomInteger 200) (Variables|Default|GetFlickerFrequency) :!label _label
    (:>
      (Rendering|SetVisibility _light true true :!label _label_2)
      (Rendering|SetVisibility _pointlight true false))
    (:==
      (goto _label_2))
    (:<
      (Rendering|SetVisibility _light false true)
      (Rendering|SetVisibility _pointlight false false)))
  (Utilities|FlowControl|Delay 0.01)
  (goto _label))

(fn ConstructionScript
  (|CallParentFunction))