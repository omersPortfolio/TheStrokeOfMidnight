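; BP_RedLamp is an interactable lamp that flickers at random when its switch flag is set.
; On BeginPlay it reads IsSwitchFlipped once, hiding Light and PointLight if false.
; If true, an endless short-Delay loop compares a random integer to FlickerFrequency, showing both components when equal or above and hiding them when below.
; A higher FlickerFrequency therefore keeps the lamp dark more often.
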(event OnComponentActivated(Light)
  (params (Component :type Actor%20Component%20Object%20Reference) (bReset :type Boolean)))

(event EventBeginPlay
  (bind _light (Variables|Default|GetLight))
  (bind _pointlight (Variables|Default|GetPointLight))
  (if (Variables|Default|GetIsSwitchFlipped)
    (Math|Integer|CompareInt (Math|Random|RandomInteger 200) (Variables|Default|GetFlickerFrequency) :!label _label
      (:>
        (Rendering|SetVisibility _light true true :!label _label_2)
        (Rendering|SetVisibility _pointlight true false))
      (:==
        (goto _label_2))
      (:<
        (Rendering|SetVisibility _light false true)
        (Rendering|SetVisibility _pointlight false false)))
    (Utilities|FlowControl|Delay 0.01)
    (goto _label)
    (else
      (Rendering|SetVisibility (Variables|Default|GetLight) false true)
      (Rendering|SetVisibility (Variables|Default|GetPointLight) false false))))

(fn ConstructionScript
  (|CallParentFunction))