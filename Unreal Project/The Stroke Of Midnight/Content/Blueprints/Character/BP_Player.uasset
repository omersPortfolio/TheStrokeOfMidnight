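; BP_Player is the player character Blueprint, holding temporary debug inputs and simple status queries.
; Key 5 stands in for a pause menu, returning to the main menu behind a loading screen by streaming in MainMenuMap, unpossessing, and unloading the saved level and Area_1.
; Key 2 or the right shoulder button makes a long-range "Player"-tagged noise to trigger AI.
; IsDead defers to the HealthComponent, while IsActorPlayer always returns true.
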(event Input|KeyboardEvents|2
  (params (Key :type Key%20Structure :default "None"))
  ;[1 1 1] DEBUG: Making noise to trigger AI
  (:Pressed
    (Class|Actor|MakeNoise 1.0 self (Transformation|GetActorLocation) 1e+05 "Player")))

(event Input|GamepadEvents|GamepadRightShoulder
  (params (Key :type Key%20Structure :default "None"))
  ;[1 1 1] DEBUG: Making noise to trigger AI
  (:Pressed
    (Class|Actor|MakeNoise 1.0 self (Transformation|GetActorLocation) 1e+05 "Player")))

(event Input|KeyboardEvents|5
  (params (Key :type Key%20Structure :default "None"))
  ;[1 1 1] DEBUG: Go To Main Menu. Will remain until Pause Menu is made.
  (:Pressed
    (bind _returnvalue (UserInterface|CreateWidget "/Game/Blueprints/UI/Widgets/WBP_LoadingScreen.WBP_LoadingScreen_C" (Game|GetPlayerController 0)))
    (UserInterface|Viewport|AddtoViewport _returnvalue 0)
    (Game|UnloadStreamLevel(byName) "MainMenuMap" true)
    (Game|LoadStreamLevel(byName) "MainMenuMap" true true)
    (Pawn|UnPossess (Game|GetPlayerController 0))
    (Utilities|FlowControl|Delay 1.5)
    (Viewport|RemoveAllWidgets)
    (Game|UnloadStreamLevel(byName) (Utilities|String|StringToName (.levelname (Variables|/Script/TheStrokeOfMidnight.PSaveGame|GetLevelData (Variables|/Script/TheStrokeOfMidnight.PGameInstance|GetSaveGameInstance (Variables|Default|GetGameInstance))))) false)
    (Game|UnloadStreamLevel(byName) "Area_1" false)))

(fn ConstructionScript)

(fn IsDead
  (return (Class|PHealthComponent|IsDead (Variables|Default|GetHealthComponent))))

(fn IsActorPlayer
  (return true))